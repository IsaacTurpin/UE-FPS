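; BP_Weapon is an FPS weapon Blueprint that plays the cosmetic effects of a shot, skipped on dedicated servers.
; FireEffects picks the first- or third-person mesh and reads its muzzle socket location.
; It lazily spawns and reuses fire, impact and decal helper actors attached to that mesh, passing each the impact point, normal and surface type.
; It then plays the fire sound and montage.
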(event EventFireEffects
  (params (ImpactPoint :type Vector%20%28by%20ref%29 :default "0, 0, 0") (ImpactNormal :type Vector%20%28by%20ref%29 :default "0, 0, 0") (ImpactSurfaceType :type EPhysicalSurface%20Enum :default "SurfaceType_Default") (bIsFirstPerson :type Boolean))
  (Variables|Default|SetIs%20First%20Person bIsFirstPerson)
  (if (not (Networking|IsDedicatedServer))
    (Variables|Default|SetImpact%20Points (Utilities|Array|MakeArray ImpactPoint))
    (Variables|Default|SetImpact%20Normals (Utilities|Array|MakeArray ImpactNormal))
    (Variables|Default|SetImpact%20Surface%20Types (Utilities|Array|MakeArray ImpactSurfaceType))
    (Utilities|FlowControl|Sequence
      (:then_0
        (if (Variables|Default|GetIs%20First%20Person)
          (Variables|Default|SetSkeletal%20Mesh (Variables|Default|GetMesh1P))
          (else
            (Variables|Default|SetSkeletal%20Mesh (Variables|Default|GetMesh3P)))))
      (:then_1
        (Variables|Default|SetMuzzle%20Position (Transformation|GetSocketLocation (Variables|Default|GetSkeletal%20Mesh) (Variables|Default|GetMuzzle%20Socket%20Name))))
      (:then_2
        (Utilities|FlowControl|Sequence
          (:then_0
            (Utilities|IsValid (Variables|Default|GetWeapon%20Fire)
              (:Is%20Valid
                _)
              (:Is%20Not%20Valid
                (bind _returnvalue (Game|SpawnActorfromClass "/Game/Effects/Blueprints/B_WeaponFire.B_WeaponFire_C" (Math|Transform|MakeTransform "0, 0, 0") "Undefined" "OverrideRootScale" 0 (Variables|Default|GetSkeletal%20Mesh) true (Variables|Default|GetShell%20Eject%20System) true (Variables|Default|GetMuzzle%20Flash%20System) true (Variables|Default|GetTracer%20System) (Variables|Default|GetShell%20Eject%20Mesh) 0))
                (bind _output_get (Variables|Default|SetWeapon%20Fire _returnvalue))
                (Transformation|AttachComponentToComponent _output_get (Variables|Default|GetSkeletal%20Mesh) "None" "KeepRelative" "KeepRelative" "KeepRelative" true)))
            (Variables|/Game/Effects/Blueprints/B_WeaponFire.B_WeaponFire_C|SetImpactPositions (Variables|Default|GetWeapon%20Fire) (Variables|Default|GetImpact%20Points))
            (Variables|/Game/Effects/Blueprints/B_WeaponFire.B_WeaponFire_C|SetImpactNormals (Variables|Default|GetWeapon%20Fire) (Variables|Default|GetImpact%20Normals))
            (Variables|/Game/Effects/Blueprints/B_WeaponFire.B_WeaponFire_C|SetImpactSurfaceTypes (Variables|Default|GetWeapon%20Fire) (Variables|Default|GetImpact%20Surface%20Types))
            (Default|Fire (Variables|Default|GetWeapon%20Fire) (Variables|Default|GetIs%20First%20Person)))
          (:then_1
            (Utilities|IsValid (Variables|Default|GetWeapon%20Impacts)
              (:Is%20Valid
                _)
              (:Is%20Not%20Valid
                (bind _returnvalue_2 (Game|SpawnActorfromClass "/Game/Effects/Blueprints/B_WeaponImpacts.B_WeaponImpacts_C" (Math|Transform|MakeTransform "0, 0, 0") "Undefined" "OverrideRootScale" 0 5e+02 0))
                (bind _output_get_2 (Variables|Default|SetWeapon%20Impacts _returnvalue_2))
                (Transformation|AttachComponentToComponent _output_get_2 (Variables|Default|GetSkeletal%20Mesh) "None" "KeepRelative" "KeepRelative" "KeepRelative" true)))
            (Variables|/Game/Effects/Blueprints/B_WeaponImpacts.B_WeaponImpacts_C|SetImpactPositions (Variables|Default|GetWeapon%20Impacts) (Variables|Default|GetImpact%20Points))
            (Variables|/Game/Effects/Blueprints/B_WeaponImpacts.B_WeaponImpacts_C|SetImpactNormals (Variables|Default|GetWeapon%20Impacts) (Variables|Default|GetImpact%20Normals))
            (Variables|/Game/Effects/Blueprints/B_WeaponImpacts.B_WeaponImpacts_C|SetImpactSurfaceTypes (Variables|Default|GetWeapon%20Impacts) (Variables|Default|GetImpact%20Surface%20Types))
            (Variables|/Game/Effects/Blueprints/B_WeaponImpacts.B_WeaponImpacts_C|SetMuzzlePosition (Variables|Default|GetWeapon%20Impacts) (Variables|Default|GetMuzzle%20Position))
            (Default|Fire (Variables|Default|GetWeapon%20Impacts) (Variables|Default|GetIs%20First%20Person)))
          (:then_2
            (Utilities|IsValid (Variables|Default|GetWeapon%20Decals)
              (:Is%20Valid
                _)
              (:Is%20Not%20Valid
                (bind _returnvalue_3 (Game|SpawnActorfromClass "/Game/Effects/Blueprints/B_WeaponDecals.B_WeaponDecals_C" (Math|Transform|MakeTransform "0, 0, 0") "Undefined" "OverrideRootScale" 0 0))
                (bind _output_get_3 (Variables|Default|SetWeapon%20Decals _returnvalue_3))
                (Transformation|AttachComponentToComponent _output_get_3 (Variables|Default|GetSkeletal%20Mesh) "None" "KeepRelative" "KeepRelative" "KeepRelative" true)))
            (Variables|/Game/Effects/Blueprints/B_WeaponDecals.B_WeaponDecals_C|SetImpactPositions (Variables|Default|GetWeapon%20Decals) (Variables|Default|GetImpact%20Points))
            (Variables|/Game/Effects/Blueprints/B_WeaponDecals.B_WeaponDecals_C|SetImpactNormals (Variables|Default|GetWeapon%20Decals) (Variables|Default|GetImpact%20Normals))
            (Variables|/Game/Effects/Blueprints/B_WeaponDecals.B_WeaponDecals_C|SetImpact%20Surface%20Types (Variables|Default|GetWeapon%20Decals) (Variables|Default|GetImpact%20Surface%20Types))
            (Default|Fire (Variables|Default|GetWeapon%20Decals) (Variables|Default|GetMuzzle%20Position)))
          (:then_3
            (Audio|PlaySoundatLocation (Variables|Default|GetWeapon%20Fire%20Sound) (Transformation|GetActorLocation) "0, 0, 0" 1.0 1.0 0.0 0 0 0 0)
            (Animation|Montage|PlayMontage (Variables|Default|GetSkeletal%20Mesh) (Variables|Default|GetWeapon%20Fire%20Montage))))))))

(fn ConstructionScript)